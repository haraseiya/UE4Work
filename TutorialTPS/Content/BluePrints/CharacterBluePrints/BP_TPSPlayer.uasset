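; Third-person shooter player character with movement, look, sprint, aiming and automatic fire.
; Aiming notifies ShooterAnimBP and drives an ArmLength timeline meant for spring arm zoom and walk speed changes.
; Holding Fire loops Shoot on a timer, tracing from the camera with debug drawing and sound, without using the hit.
; BeginPlay gathers all Weapon_BP actors in the level; weapon swap input only compares the axis value.
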(event Custom|Shoot
  (bind _returnvalue (Game|GetPlayerCameraManager 0))
  (bind _returnvalue_2 (Transformation|GetActorLocation _returnvalue))
  ;[1 1 1] Fire
  (Collision|LineTraceByChannel _returnvalue_2 (+ _returnvalue_2 (* (Math|Vector|GetForwardVector (Transformation|GetActorRotation _returnvalue)) (Variables|Weapon|GetBulletRange))) "TraceTypeQuery1" false 0 "ForDuration")
  (Audio|PlaySound2D "/Engine/EditorSounds/Notifications/CompileFailed.CompileFailed" 1.0 1.0 0.0 0 0))

(event EventBeginPlay
  (Utilities|FlowControl|Sequence
    (:then_0
      (Variables|Default|SetmyAnimBP (.AsShooter%20Anim%20BP (Utilities|Casting|CastToShooterAnimBP (Components|SkeletalMesh|GetAnimInstance (Variables|Character|GetMesh))))))
    (:then_1
      (bind _outactors (Actor|GetAllActorsOfClass "/Game/BluePrints/ActorBlueprints/Weapon_BP.Weapon_BP_C"))
      (for _array_element _outactors
        (Utilities|Array|Add (Variables|Weapon|GetWeapons) _array_element))
      (bind _output_get (Variables|Weapon|SetWeaponIndexLength (Utilities|Array|Length (Variables|Weapon|GetWeapons))))
      (Development|PrintString (Utilities|String|ToString(Integer) _output_get)))
    (:then_2
      (Variables|Weapon|SetMyWeapon (Utilities|Array|MakeArray (Utilities|Array|Get(acopy) (Variables|Weapon|GetWeapons)))))))

(event Input|ActionEvents|InputActionAiming
  (params (Key :type Key%20Structure :default "None"))
  (bind _armlength (Variables|Default|GetArmLength))
  (bind _myanimbp (Variables|Default|GetmyAnimBP))
  (:Pressed
    (Class|CharactertoAnimInterface|IsAiming?(Message) _myanimbp true)
    (Audio|Components|Audio|Play _armlength))
  (:Released
    (Class|CharactertoAnimInterface|IsAiming?(Message) _myanimbp false)
    (Utilities|String|Reverse _armlength)))

(event Input|ActionEvents|InputActionSprint
  (params (Key :type Key%20Structure :default "None"))
  (bind _charactermovement (Variables|Character|GetCharacterMovement))
  (:Pressed
    (Variables|/Script/Engine.CharacterMovementComponent|SetMaxWalkSpeed _charactermovement 6e+02))
  (:Released
    (Variables|/Script/Engine.CharacterMovementComponent|SetMaxWalkSpeed _charactermovement 3.5e+02)))

(event Input|ActionEvents|InputActionFire
  (params (Key :type Key%20Structure :default "None"))
  ;[1 1 1] Fire
  (:Pressed
    (CallFunction|Shoot)
    (Utilities|Time|SetTimerbyFunctionName 0 "Shoot" 0.1 true))
  (:Released
    (Utilities|Time|ClearTimerbyFunctionName 0 "Shoot")))

(event Input|AxisEvents|InputAxisMoveForward
  (params (AxisValue :type Float%20%28single-precision%29))
  (Pawn|Input|AddMovementInput (Math|Vector|GetForwardVector (Transformation|GetActorRotation)) AxisValue false))

(event Input|AxisEvents|InputAxisMoveRight
  (params (AxisValue :type Float%20%28single-precision%29))
  (Pawn|Input|AddMovementInput (Math|Vector|GetRightVector (Transformation|GetActorRotation)) AxisValue false))

(event Input|AxisEvents|InputAxisTurn
  (params (AxisValue :type Float%20%28single-precision%29))
  (Pawn|Input|AddControllerYawInput AxisValue))

(event Input|AxisEvents|InputAxisLookUp
  (params (AxisValue :type Float%20%28single-precision%29))
  (Pawn|Input|AddControllerPitchInput AxisValue))

(event Input|AxisEvents|InputAxisSwapWeapon
  (params (AxisValue :type Float%20%28single-precision%29))
  (bind _output_get (Variables|Weapon|SetWheelAxisValue AxisValue))
  (Math|Float|CompareFloat _output_get 0.0))

(fn ConstructionScript)