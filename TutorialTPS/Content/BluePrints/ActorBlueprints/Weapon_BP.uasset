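; Weapon_BP is a weapon actor that holds a gun mesh along with damage, fire rate and ammo stats.
; SetAttachment casts player pawn 0 to BP_TPSPlayer and attaches the gun mesh to a given socket on that character's mesh, keeping relative transforms.
; Simple setter and getter functions write and read the weapon stats, while the event graph and construction script contain no logic.
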(event EventBeginPlay)

(event Collision|EventActorBeginOverlap
  (params (OtherActor :type Actor%20Object%20Reference)))

(event EventTick
  (params (DeltaSeconds :type Float%20%28single-precision%29)))

(fn ConstructionScript)

(fn SetAttachment
  (params (SocketName :type Name))
  (Transformation|AttachComponentToComponent (Variables|Default|GetGunMesh) (Variables|/Script/Engine.Character|GetMesh (.AsBP%20TPSPlayer (Utilities|Casting|CastToBP_TPSPlayer (Game|Player|GetPlayerPawn 0)))) SocketName "KeepRelative" "KeepRelative" "KeepRelative" true))

(fn SetWeaponSpec
  (params (Damage :type Float%20%28single-precision%29) (Firerate :type Float%20%28single-precision%29) (Ammo :type Integer))
  (Variables|Default|SetDamage Damage)
  (Variables|Default|SetFireRate Firerate)
  (Variables|Default|SetAmmo Ammo))

(fn GetWeponSpec
  (return (Variables|Default|GetDamage) (Variables|Default|GetFireRate) (Variables|Default|GetAmmo)))